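; Attack ability executor for the card system that previews which map tiles an ability affects; no damage is applied here.
; On begin, it shows the forward-facing pattern and caches the KK player controller.
; GetAffectedTiles rotates the character's relative tile pattern, resolves it through the map and colors the resulting tiles red.
; Rotate-direction input hides the current tiles and redraws the pattern in the chosen direction.
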(event `self.BeginAbility`
  (`self.GetAffectedTiles` "ERD_Forward")
  (bind _asbp_kkplayer_controller (cast `/Game/Player/BP_KKPlayerController` (`GameplayStatics.GetPlayerController` 0)))
  (set `self.KKPlayer Controller` _asbp_kkplayer_controller))

(event `EnhancedInput|/Game/Player/Input/Actions/IA_RotateDirection`
  (params (ActionValue :type "Float (double-precision)") (ElapsedSeconds :type "Float (double-precision)") (TriggeredSeconds :type "Float (double-precision)") (InputAction :type "InputAction Object Reference" :default "/Game/Player/Input/Actions/IA_RotateDirection.IA_RotateDirection"))
  (:`Started`
    (`/Game/Player/BP_KKPlayerController.HideTiles` (`self.KKPlayer Controller`))
    (`self.GetAffectedTiles` (`self.GetRotationFromInt` (`KismetMathLibrary.FTrunc` ActionValue)))))

(fn `GetAffectedTiles`
  (params (RotationDirection :type "ERotationDirection Enum" :default "ERD_Forward"))
  (bind _character (`self.Character`))
  (bind _returnvalue (message `AreaModifierInterface.GetAffectedTiles` _character (`self.Index`)))
  (bind _returnvalue_2 (`KKCharacter.RotateDirections` _character _returnvalue RotationDirection))
  (bind _returnvalue_3 (`KKMap.GetTilesByDirection` (`self.GetMap`) (`self.Character`) _returnvalue_2 "TSP_AllTiles"))
  (for _array_element _returnvalue_3
    (`KKTile.SetTileColor` _array_element "Red")))

(fn `UserConstructionScript`)