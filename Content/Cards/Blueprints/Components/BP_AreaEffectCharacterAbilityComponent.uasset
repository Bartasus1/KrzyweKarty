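; Character ability component for area-effect abilities that previews the affected tiles on the map.
; On begin, it fetches the owner character's affected tile pattern for the ability index and enables tick.
; The rotate input re-fetches that pattern and rotates it to the chosen direction.
; Each tick clears highlights and paints the resolved tiles red; finishing stops tick and clears them.
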(event `self.BeginAbility`
  (`parent.BeginAbility`)
  (bind _returnvalue (message `AreaModifierInterface.GetAffectedTiles` (`self.OwnerCharacter`) (`self.AbilityIndex`)))
  (set `self.AffectedTiles` _returnvalue)
  (`self.SetComponentTickEnabled` true))

(event `self.FinishAbility`
  (params (bWasCancelled :type Boolean))
  (`self.SetComponentTickEnabled` false)
  (`KKMap.ClearTilesHighlights` (`self.GetMap`)))

(event `EnhancedInput|/Game/Player/Input/Actions/IA_RotateDirection`
  (params (ActionValue :type "Float (double-precision)") (ElapsedSeconds :type "Float (double-precision)") (TriggeredSeconds :type "Float (double-precision)") (InputAction :type "InputAction Object Reference" :default "/Game/Player/Input/Actions/IA_RotateDirection.IA_RotateDirection"))
  (:`Started`
    (bind _returnvalue (message `AreaModifierInterface.GetAffectedTiles` (`self.OwnerCharacter`) (`self.AbilityIndex`)))
    (bind _output_get (set `self.AffectedTiles` _returnvalue))
    (`KKGameStatics.RotateDirections` _output_get (select `int` (- (`KismetMathLibrary.FTrunc` ActionValue) 1) :`0` "ERD_Left" :`1` "ERD_Forward" :`2` "ERD_Right" :`3` "ERD_Backward" :!type "ERotationDirection Enum"))))

(event `self.ReceiveTick`
  (params (DeltaSeconds :type "Float (single-precision)"))
  (bind _returnvalue (`self.GetMap`))
  (`KKMap.ClearTilesHighlights` _returnvalue)
  (bind _returnvalue_2 (`KKMap.GetTilesByDirection` _returnvalue (`self.OwnerCharacter`) (`self.AffectedTiles`) "TSP_AllTiles"))
  (for _array_element _returnvalue_2
    (`KKTile.SetTileColor` _array_element "Red")))