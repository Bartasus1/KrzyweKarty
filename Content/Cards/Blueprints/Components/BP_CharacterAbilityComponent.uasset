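; BP_CharacterAbilityComponent is an ability component that lets the player confirm or abort the owning character's ability.
; Beginning the ability runs the parent logic, enables input on the owner character and adds a high-priority Enhanced Input mapping context.
; The confirm action finishes the ability normally and the abort action finishes it as cancelled.
; Finishing runs the parent logic, disables the character's input and removes the mapping context.
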(event `self.BeginAbility`
  (bind _returnvalue (`self.GetPlayerController`))
  (`parent.BeginAbility`)
  (`Actor.EnableInput` (`self.OwnerCharacter`) _returnvalue)
  (`EnhancedInputSubsystemInterface.AddMappingContext` (pcsubsystem `EnhancedInputLocalPlayerSubsystem` _returnvalue) "/Game/Player/Input/IMC_CharacterAbilityContext.IMC_CharacterAbilityContext" 1000 (struct)))

(event `self.FinishAbility`
  (params (bWasCancelled :type Boolean))
  (bind _returnvalue (`self.GetPlayerController`))
  (`parent.FinishAbility` bWasCancelled)
  (`Actor.DisableInput` (`self.OwnerCharacter`) _returnvalue)
  (`EnhancedInputSubsystemInterface.RemoveMappingContext` (pcsubsystem `EnhancedInputLocalPlayerSubsystem` _returnvalue) "/Game/Player/Input/IMC_CharacterAbilityContext.IMC_CharacterAbilityContext" (struct)))

(event `EnhancedInput|/Game/Player/Input/Actions/IA_Confirm`
  (params (ActionValue :type Boolean) (ElapsedSeconds :type "Float (double-precision)") (TriggeredSeconds :type "Float (double-precision)") (InputAction :type "InputAction Object Reference" :default "/Game/Player/Input/Actions/IA_Confirm.IA_Confirm"))
  (:`Started`
    (`self.FinishAbility` false)))

(event `EnhancedInput|/Game/Player/Input/Actions/IA_Abort`
  (params (ActionValue :type Boolean) (ElapsedSeconds :type "Float (double-precision)") (TriggeredSeconds :type "Float (double-precision)") (InputAction :type "InputAction Object Reference" :default "/Game/Player/Input/Actions/IA_Abort.IA_Abort"))
  (:`Started`
    (`self.FinishAbility` true)))