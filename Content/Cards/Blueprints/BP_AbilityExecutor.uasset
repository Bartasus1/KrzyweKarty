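; BP_AbilityExecutor is an actor that runs the lifecycle of a character's active ability, apparently as a base for specific abilities.
; BeginAbility asks the Character whether the ability at Index is usable, then either calls ShowActiveAbilityState(false) or ends it through SREndAbility.
; Confirm and Abort inputs call SRExecuteAbility and SREndAbility.
; ExecuteAbility is an empty hook, and EndAbility destroys the actor.
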(event `self.BeginAbility`
  (bind _returnvalue (`KKCharacter.CanUseActiveAbility` (`self.Character`) (`self.Index`)))
  (if _returnvalue
    (`KKCharacter.ShowActiveAbilityState` (`self.Character`) false)
    (else
      (`self.SR_EndAbility`))))

(event `self.ExecuteAbility`)

(event `self.EndAbility`
  (`self.K2_DestroyActor`))

(event `EnhancedInput|/Game/Player/Input/Actions/IA_Abort`
  (params (ActionValue :type Boolean) (ElapsedSeconds :type "Float (double-precision)") (TriggeredSeconds :type "Float (double-precision)") (InputAction :type "InputAction Object Reference" :default "/Game/Player/Input/Actions/IA_Abort.IA_Abort"))
  (:`Triggered`
    (`self.SR_EndAbility`)))

(event `EnhancedInput|/Game/Player/Input/Actions/IA_Confirm`
  (params (ActionValue :type Boolean) (ElapsedSeconds :type "Float (double-precision)") (TriggeredSeconds :type "Float (double-precision)") (InputAction :type "InputAction Object Reference" :default "/Game/Player/Input/Actions/IA_Confirm.IA_Confirm"))
  (:`Triggered`
    (`self.SR_ExecuteAbility`)))

(fn `UserConstructionScript`)