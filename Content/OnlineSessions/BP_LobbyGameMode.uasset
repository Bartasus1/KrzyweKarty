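; BP_LobbyGameMode is the game mode for the online session lobby, tracking joined players and their readiness to start.
; On PostLogin it gives each BP_LobbyPlayerController an ID from the current player count and stores it.
; OnFractionSelected records the player's ID in ReadyToStart and reports whether at least two entries are present.
; ShowStartingInfo relays the starting info call to every stored controller.
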(event `self.K2_PostLogin`
  (params (NewPlayer :type "PlayerController Object Reference"))
  (bind _asbp_lobby_player_controller (cast `/Game/OnlineSessions/BP_LobbyPlayerController` NewPlayer))
  (bind _returnvalue (`self.GetNumPlayers`))
  (set `/Game/OnlineSessions/BP_LobbyPlayerController.ID` _returnvalue _asbp_lobby_player_controller)
  (`KismetArrayLibrary.Array_Add` (`self.PlayerControllers`) _asbp_lobby_player_controller))

(event `ShowStartingInfo`
  (for _array_element (`self.PlayerControllers`)
    (`/Game/OnlineSessions/BP_LobbyPlayerController.ShowStartingInfo` _array_element)))

(fn `On Fraction Selected`
  (params (PlayerID :type Integer))
  (returns (CanStartMatch :type Boolean))
  (`BlueprintSetLibrary.Set_Add` (`self.ReadyToStart`) PlayerID)
  (return (>= (`BlueprintSetLibrary.Set_Length` (`self.ReadyToStart`)) 2)))

(fn `UserConstructionScript`)