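; Lobby player controller that runs fraction (faction) selection before a match.
; On BeginPlay, the local controller shows the fraction selection widget in UI-only input mode.
; SetFraction inserts the choice into the game instance by player ID and notifies BP_LobbyGameMode.
; If that returns true, it calls the game mode's ShowStartingInfo and server-travels to GameLevel_01; its own ShowStartingInfo event displays the start-game widget.
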(event `self.ReceiveBeginPlay`
  (if (`self.IsLocalPlayerController`)
    (bind _returnvalue (`|CreateWidget` "/Game/UI/Lobby/WB_FractionSelection.WB_FractionSelection_C"))
    (`WidgetBlueprintLibrary.SetInputMode_UIOnlyEx` self _returnvalue)
    (`UserWidget.AddToViewport` _returnvalue 0)))

(event `SetFraction`
  (params (Fraction :type "Fraction Class Reference"))
  (bind _askrzywe_karty_game_instance (cast `/Game/KrzyweKartyGameInstance` (`GameplayStatics.GetGameInstance`)))
  (`KismetArrayLibrary.Array_Insert` (`/Game/KrzyweKartyGameInstance.PlayersFractions` _askrzywe_karty_game_instance) Fraction (- (`self.ID`) 1))
  (bind _asbp_lobby_game_mode (cast `/Game/OnlineSessions/BP_LobbyGameMode` (`GameplayStatics.GetGameMode`)))
  (bind _canstartmatch (`/Game/OnlineSessions/BP_LobbyGameMode.On Fraction Selected` _asbp_lobby_game_mode (`self.ID`)))
  (if _canstartmatch
    (`/Game/OnlineSessions/BP_LobbyGameMode.ShowStartingInfo` _asbp_lobby_game_mode)
    (`KismetSystemLibrary.ExecuteConsoleCommand` "servertravel /Game/Levels/GameLevel_01" self)))

(event `ShowStartingInfo`
  (bind _returnvalue (`|CreateWidget` "/Game/UI/Lobby/WB_StartGame.WB_StartGame_C"))
  (`UserWidget.AddToViewport` _returnvalue 0))

(fn `UserConstructionScript`)