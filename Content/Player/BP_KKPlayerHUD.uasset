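; BP_KKPlayerHUD is the player HUD that puts the log panel and turn-change notices on screen.
; On BeginPlay it creates WB_LogPanel and adds it to the viewport.
; OnTurnChange removes any previous turn widget, then creates and shows a WB_RoundEndWidget for the owning player, passing in whether it is their turn.
; A disconnected branch that would show WB_CurrentPlayerTurnWidget never runs.
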(event `self.ReceiveBeginPlay`
  (bind _returnvalue (`|CreateWidget` "/Game/UI/WB_LogPanel.WB_LogPanel_C"))
  (`UserWidget.AddToViewport` _returnvalue 0))

(event `self.OnTurnChange`
  (params (bIsMyTurn :type Boolean))
  (bind _changeturnwidget (`self.ChangeTurnWidget`)
    (:`then`
      (`Widget.RemoveFromParent` _changeturnwidget))
    (:`else`
      _))
  (bind _returnvalue (`|CreateWidget` "/Game/UI/WB_RoundEndWidget.WB_RoundEndWidget_C" (`self.GetOwningPlayerController`) bIsMyTurn))
  (bind _output_get (set `self.ChangeTurnWidget` _returnvalue))
  (`UserWidget.AddToViewport` _output_get 0))

(fn `UserConstructionScript`)