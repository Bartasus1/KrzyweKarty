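; BP_KKPlayer is a player actor that pans across the world and zooms its camera.
; BeginPlay registers the default Enhanced Input mapping context for player zero.
; Zoom input adjusts the camera's field of view within a clamped range rather than moving the camera.
; Move input teleports the actor horizontally without sweeping, undoing any step that leaves a fixed box centred on the world origin.
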(event `self.ReceiveBeginPlay`
  (`EnhancedInputSubsystemInterface.AddMappingContext` (pcsubsystem `EnhancedInputLocalPlayerSubsystem` (`GameplayStatics.GetPlayerController` 0)) "/Game/Player/Input/IMC_DefaultPlayerContext.IMC_DefaultPlayerContext" 0 (struct)))

(event `EnhancedInput|/Game/Player/Input/Actions/IA_Zoom`
  (params (ActionValue :type "Float (double-precision)") (ElapsedSeconds :type "Float (double-precision)") (TriggeredSeconds :type "Float (double-precision)") (InputAction :type "InputAction Object Reference" :default "/Game/Player/Input/Actions/IA_Zoom.IA_Zoom"))
  (:`Triggered`
    (`CameraComponent.SetFieldOfView` (`self.Camera`) (`KismetMathLibrary.FClamp` (+ (`CameraComponent.FieldOfView` (`self.Camera`)) (* ActionValue 5.0)) 45.0 130.0))))

(event `EnhancedInput|/Game/Player/Input/Actions/IA_Move`
  (params (ActionValue :type "Vector2D Structure") (ElapsedSeconds :type "Float (double-precision)") (TriggeredSeconds :type "Float (double-precision)") (InputAction :type "InputAction Object Reference" :default "/Game/Player/Input/Actions/IA_Move.IA_Move"))
  (bind _returnvalue (`KismetMathLibrary.Conv_Vector2DToVector` (* ActionValue 5.0)))
  (:`Triggered`
    (if (`KismetMathLibrary.IsPointInBox` (`self.K2_GetActorLocation`) (0.0 0.0 0.0) (1500.0 1000.0 1000.0))
      (`self.K2_AddActorWorldOffset` _returnvalue false true)
      (if (not (`KismetMathLibrary.IsPointInBox` (`self.K2_GetActorLocation`) (0.0 0.0 0.0) (1500.0 1000.0 1000.0)))
        (`self.K2_AddActorWorldOffset` (* _returnvalue -1.0) false true)))))

(fn `UserConstructionScript`)