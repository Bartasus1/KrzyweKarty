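; Player controller for a turn-based tile game, handling camera look, character selection, abilities and hold-to-end-turn with HUD progress.
; After selection, an async search picks a target whose tile status gameplay tag chooses a summon, move or attack action object.
; Abilities selected from the widget spawn an ability actor and push a higher-priority input mapping context.
; ShowAbility1Tiles is an unfinished stub that loops over characters' tiles without effect.
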(event `EnhancedInput|/Game/Player/Input/Actions/IA_Look`
  (params (ActionValue :type "Vector2D Structure") (ElapsedSeconds :type "Float (double-precision)") (TriggeredSeconds :type "Float (double-precision)") (InputAction :type "InputAction Object Reference" :default "/Game/Player/Input/Actions/IA_Look.IA_Look"))
  (bind (_x _y) (`KismetMathLibrary.BreakVector2D` ActionValue))
  ;[1 1 1] Inputs
  (:`Triggered`
    (`self.AddYawInput` _x)
    (if (not (`self.bLockPitch`))
      (`self.AddPitchInput` _y))))

(event `Key|LeftControl`
  (params (Key :type "Key Structure"))
  ;[1 1 1] Inputs
  (:`Pressed`
    (set `self.bLockPitch` true))
  (:`Released`
    (set `self.bLockPitch` false)))

(event `CharacterAddToMap`
  (params (TileID :type Byte) (Character :type "KKCharacter Object Reference"))
  ;[1 1 1] Server Functions
  (bind _returnvalue (`|GenericCreateObject` "/Script/KrzyweKarty.SummonAction" TileID Character))
  (`Action.TryBeginAction` _returnvalue))

(event `EnhancedInput|/Game/Player/Input/Actions/IA_ChangeTurn`
  (params (ActionValue :type Boolean) (ElapsedSeconds :type "Float (double-precision)") (TriggeredSeconds :type "Float (double-precision)") (InputAction :type "InputAction Object Reference" :default "/Game/Player/Input/Actions/IA_ChangeTurn.IA_ChangeTurn"))
  ;[1 1 1] Inputs
  (:`Triggered`
    (if (`self.bIsMyTurn`)
      (`ProgressBar.SetPercent` (`self.GetChangeTurnProgressbar`) 1.0)
      (`self.ChangeTurn`)))
  (:`Ongoing`
    (if (`self.bIsMyTurn`)
      (`ProgressBar.SetPercent` (`self.GetChangeTurnProgressbar`) ElapsedSeconds)))
  (:`Completed`
    (`ProgressBar.SetPercent` (`self.GetChangeTurnProgressbar`) 0.0)))

(event `MoveCharacter`
  (params (TileID :type Byte) (Character :type "KKCharacter Object Reference"))
  ;[1 1 1] Server Functions
  (bind _returnvalue (`|GenericCreateObject` "/Script/KrzyweKarty.MoveAction" TileID Character))
  (`Action.TryBeginAction` _returnvalue))

(event `self.ReceiveBeginPlay`
  ;[1 1 1] Inputs
  (`parent.ReceiveBeginPlay`)
  (`WidgetBlueprintLibrary.SetFocusToGameViewport`))

(event `AttackCharacter`
  (params (TileID :type Byte) (Character :type "KKCharacter Object Reference"))
  ;[1 1 1] Server Functions
  (bind _returnvalue (`KKMap.GetCharacterAtIndex` (`self.GetMap`) TileID))
  (bind _returnvalue_2 (`|GenericCreateObject` "/Script/KrzyweKarty.AttackAction" _returnvalue Character))
  (`Action.TryBeginAction` _returnvalue_2))

(event `EnhancedInput|/Game/Player/Input/Actions/IA_SelectCharacter`
  (params (ActionValue :type Boolean) (ElapsedSeconds :type "Float (double-precision)") (TriggeredSeconds :type "Float (double-precision)") (InputAction :type "InputAction Object Reference" :default "/Game/Player/Input/Actions/IA_SelectCharacter.IA_SelectCharacter"))
  ;[1 1 1] Inputs
  (:`Started`
    (`KKGameStatics.HideTiles`)
    (bind _returnvalue (`self.SelectCharacter`))
    (if _returnvalue
      (`self.OnCharacterSelection`)
      (bind _selectable (`FindSelectableAsync.FindSelectableAsync` self false)
        (:`SelectableFound`
          (`self.MakeActionForTile` _selectable))
        (:`SelectableNotFound`
          (`KKGameStatics.HideTiles`))))))

(event `UseCharacterAbility`
  (params (Character :type "KKCharacter Object Reference") (Index :type Byte))
  ;[1 1 1] Server Functions
  (bind _returnvalue (`|SpawnActorFromClass` (`KKCharacter.GetAbilityClass` Character Index) (`KismetMathLibrary.MakeTransform` (0.0 0.0 0.0)) "Undefined" "MultiplyWithRoot" null Character Index null))
  (bind _output_get (set `self.CurrentAbilityActor` _returnvalue))
  (`AbilityActor.BeginAbility` _output_get))

(event `EnhancedInput|/Game/Player/Input/Actions/IA_UnSelectCharacter`
  (params (ActionValue :type Boolean) (ElapsedSeconds :type "Float (double-precision)") (TriggeredSeconds :type "Float (double-precision)") (InputAction :type "InputAction Object Reference" :default "/Game/Player/Input/Actions/IA_UnSelectCharacter.IA_UnSelectCharacter"))
  ;[1 1 1] Inputs
  (:`Triggered`
    (bind _output_get (set `self.SelectedCharacter` null))
    (`self.ShowCharacterStats` _output_get)
    (`KKGameStatics.HideTiles`)))

(event `SelectCharacterAbility`
  (params (Index :type Byte))
  ;[1 1 1] Inputs
  (if (and (`self.bIsMyTurn`) (`KismetSystemLibrary.IsValid` (`self.SelectedCharacter`)) (not (`KismetSystemLibrary.IsValid` (`self.CurrentAbilityActor`))))
    (bind _returnvalue (`KKCharacter.CanUseAbility` (`self.SelectedCharacter`) Index))
    (if _returnvalue
      (`self.UseCharacterAbility` (`self.SelectedCharacter`) Index)
      (`self.Manage Character Ability Input` true))))

(event `ChangeTurn`
  ;[1 1 1] Server Functions
  (`KKGameState.ChangeTurn` (`self.GetGameState`)))

(fn `GetChangeTurnProgressbar`
  (returns (ChangeTurnProgressBar :type "ProgressBar Object Reference"))
  (bind _asbp_kkplayer_hud (cast `/Game/Player/BP_KKPlayerHUD` (`self.GetHUD`)))
  (return (`/Game/UI/Widgets/WB_CurrentPlayerTurnWidget.ChangeTurnProgressBar` (`/Game/Player/BP_KKPlayerHUD.CurrentPlayerTurnWidget` _asbp_kkplayer_hud))))

(fn `GetGameState`
  (returns (`Game State` :type "KKGameState Object Reference"))
  (bind _askkgame_state (cast `KKGameState` (`GameplayStatics.GetGameState`)))
  (return _askkgame_state))

(fn `GetMap`
  (returns (Map :type "KKMap Object Reference"))
  (bind _askkgame_state (cast `KKGameState` (`GameplayStatics.GetGameState`)))
  (return (`KKGameState.Map` _askkgame_state)))

(fn `MakeActionForTile`
  (params (Selectable :type "SelectableInterface Interface"))
  (locals (TileID :type Byte))
  (`|ExecutionSequence`
    (:`then_0`
      (bind _output_get (set `local.TileID` (`KismetMathLibrary.Conv_IntToByte` (`SelectableInterface.GetTilePositionID` (`local.Selectable`)))))
      (bind _returnvalue (`KKMap.GetTileAtIndex` (`self.GetMap`) _output_get))
      (bind _tilestatus (`KKTile.TileStatus` _returnvalue)
        (:`then`
          (`|SwitchGameplayTag` (`TileStatus.TileStatusTag` _tilestatus)
            (:`TileStatus.Attack`
              (`self.AttackCharacter` (`local.TileID`) (`self.SelectedCharacter`)))
            (:`TileStatus.Summon`
              (`self.CharacterAddToMap` (`local.TileID`) (`self.SelectedCharacter`)))
            (:`TileStatus.Movement`
              (`self.MoveCharacter` (`local.TileID`) (`self.SelectedCharacter`)))))
        (:`else`)))
    (:`then_1`
      (`KKGameStatics.HideTiles`))))

(fn `Manage Character Ability Input`
  (params (`Enable ?` :type Boolean))
  (if `Enable ?`
    (`self.EnableInput` (`self.SelectedCharacter`) self)
    (`EnhancedInputSubsystemInterface.AddMappingContext` (pcsubsystem `EnhancedInputLocalPlayerSubsystem` self) "/Game/Player/Input/IMC_CharacterAbilityContext.IMC_CharacterAbilityContext" 100 (struct))
    (else
      (`self.DisableInput` (`self.SelectedCharacter`) self)
      (`EnhancedInputSubsystemInterface.RemoveMappingContext` (pcsubsystem `EnhancedInputLocalPlayerSubsystem` self) "/Game/Player/Input/IMC_CharacterAbilityContext.IMC_CharacterAbilityContext" (struct)))))

(fn `Show Ability 1 Tiles`
  (`|ExecutionSequence`
    (:`then_0`
      (bind _askkgame_state (cast `KKGameState` (`GameplayStatics.GetGameState`)))
      (bind _map (`KKGameState.Map` _askkgame_state))
      (bind _returnvalue (`KKMap.GetEnemyCharactersOnMap` _map (`self.SelectedCharacter`)))
      (for _array_element _returnvalue
        (bind _returnvalue_2 (`KKMap.GetTileAtIndex` _map (`KismetMathLibrary.Conv_IntToByte` (`KKCharacter.GetTilePositionID` _array_element))))
        (`/Engine/EditorBlueprintResources/StandardMacros.IsValid` _returnvalue_2)))
    (:`then_1`
      (bind _askkgame_state_2 (cast `KKGameState` (`GameplayStatics.GetGameState`)))
      (bind _map_2 (`KKGameState.Map` _askkgame_state_2))
      (bind _returnvalue_3 (`KKMap.GetAllyCharactersOnMap` _map_2 (`self.SelectedCharacter`)))
      (for _array_element_2 _returnvalue_3
        (bind _returnvalue_4 (`KKMap.GetTileAtIndex` _map_2 (`KismetMathLibrary.Conv_IntToByte` (`KKCharacter.GetTilePositionID` _array_element_2))))
        (`/Engine/EditorBlueprintResources/StandardMacros.IsValid` _returnvalue_4)))))

(fn `UserConstructionScript`)