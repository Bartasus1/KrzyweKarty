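; Ability actor that lets the player select a character on the tile map as the ability's target.
; On begin, the owning character filters all map characters and supplies a status to mark each one's tile.
; An async selectable search on the player controller then sends the picked character to a server event and marks its tile as selected.
; Finishing requires a valid selection and hides the tiles.
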(event `self.OnBeginAbility`
  (`KKGameStatics.HideTiles`)
  (bind _returnvalue (`KKGameStatics.GetMap`))
  (bind _output_get (set `self.Map` _returnvalue))
  (bind _returnvalue_2 (`KKMap.GetAllCharactersOnMap` _output_get (`self.Character`))) ; Add Character Filtering
  (bind _returnvalue_3 (message `AreaModifierInterface.FilterCharacters` (`self.Character`) _returnvalue_2 (`self.AbilityIndex`)))
  (for _array_element _returnvalue_3
    (bind _returnvalue_4 (message `AreaModifierInterface.GetStatusForTile` (`self.Character`) _array_element (`self.AbilityIndex`)))
    (bind _returnvalue_5 (`KKMap.GetTileAtIndex` (`self.Map`) (`SelectableInterface.GetTilePositionID` _array_element)))
    (`KKTile.SetTileStatus` _returnvalue_5 _returnvalue_4))
  (bind _asbp_kkplayer_controller (cast `/Game/Player/BP_KKPlayerController` (`GameplayStatics.GetPlayerController` 0)))
  (bind _selectable (`FindSelectableAsync.FindSelectableAsync` _asbp_kkplayer_controller "ECC_GameTraceChannel1")
    (:`SelectableFound`
      (`|ExecutionSequence`
        (:`then_0`
          (bind _returnvalue_6 (`SelectableInterface.GetTilePositionID` _selectable))
          (bind _returnvalue_7 (`KKMap.GetCharacterAtIndex` (`self.Map`) _returnvalue_6))
          (`self.SetSelectedCharacter_Server` _returnvalue_7))
        (:`then_1`
          (bind _returnvalue_8 (`KKMap.GetTileAtIndex` (`self.Map`) _returnvalue_6))
          (`KKTile.SetTileStatus` _returnvalue_8 "/Game/TileStatus/SelectorSelectedTileStatus.SelectorSelectedTileStatus"))))
    (:`SelectableNotFound`
      (`KismetSystemLibrary.PrintString` "Selectable Not Found"))))

(event `self.OnFinishAbility`
  (`KKGameStatics.HideTiles`))

(event `SetSelectedCharacter_Server`
  (params (SelectedCharacter :type "KKCharacter Object Reference"))
  (set `self.SelectedCharacter` SelectedCharacter))

(fn `CanFinishAbility?`
  (returns (`Can Finish` :type Boolean))
  (return (`KismetSystemLibrary.IsValid` (`self.SelectedCharacter`))))

(fn `GetSelectedCharacter`
  (returns (ReturnValue :type "KKCharacter Object Reference"))
  (return (`self.SelectedCharacter`)))

(fn `OnAbilityFailedToFinish`
  (`KismetSystemLibrary.PrintString` "Please select a character"))

(fn `UserConstructionScript`
  (`parent.UserConstructionScript`))