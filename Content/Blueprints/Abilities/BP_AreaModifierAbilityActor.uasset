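; Ability actor for area modifier abilities that previews affected map tiles and records the characters standing on them.
; Beginning the ability shows the area facing Forward, rotate input redraws it in one of four directions, and finishing hides it.
; ShowAreaTiles gets directions and tile statuses through messages to Character, resolves rotated directions into map cells without blocking, and refreshes AffectedCharacters.
; Its own GetAffectedTiles and GetStatusForTile are empty.
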(event `EnhancedInput|/Game/Player/Input/Actions/IA_RotateDirection`
  (params (ActionValue :type "Float (double-precision)") (ElapsedSeconds :type "Float (double-precision)") (TriggeredSeconds :type "Float (double-precision)") (InputAction :type "InputAction Object Reference" :default "/Game/Player/Input/Actions/IA_RotateDirection.IA_RotateDirection"))
  (:`Triggered`
    (`KKGameStatics.HideTiles`)
    (`self.ShowAreaTiles` (select `int` (- (`KismetMathLibrary.FTrunc` ActionValue) 1) :`0` "ERD_Forward" :`1` "ERD_Right" :`2` "ERD_Backward" :`3` "ERD_Left" :!type "ERotationDirection Enum"))))

(event `self.OnBeginAbility`
  (`KKGameStatics.HideTiles`)
  (`self.ShowAreaTiles` "ERD_Forward"))

(event `self.OnFinishAbility`
  (`KKGameStatics.HideTiles`))

(event `SetAffectedCharacters`
  (params (AffectedCharacters :type "Array of KKCharacter Object Reference"))
  (set `self.AffectedCharacters` AffectedCharacters))

(fn `GetAffectedCharacters`
  (returns (ReturnValue :type "Array of KKCharacter Object Reference"))
  (return (`self.AffectedCharacters`)))

(fn `GetAffectedTiles`
  (params (Index :type Byte))
  (returns (ReturnValue :type "Array of Direction Structure"))
  (return))

(fn `GetStatusForTile`
  (params (TargetCharacter :type "KKCharacter Object Reference"))
  (returns (ReturnValue :type "TileStatus Object Reference"))
  (return null))

(fn `ShowAreaTiles`
  (params (RotationDirection :type "ERotationDirection Enum" :default "ERD_Forward"))
  (locals (MapCell :type "MapCell Structure"))
  (bind _mapcell_tile (break `MapCell` (`local.MapCell`)))
  (`KismetArrayLibrary.Array_Clear` (`self.AffectedCharacters`))
  (bind _returnvalue (message `AreaModifierInterface.GetAffectedTiles` (`self.Character`) (`self.AbilityIndex`)))
  (bind _returnvalue_2 (`KKGameStatics.RotateDirections` _returnvalue RotationDirection))
  (bind _returnvalue_3 (`KKGameStatics.GetMap`))
  (bind _returnvalue_4 (`KKMap.GetCellsByDirection` _returnvalue_3 (`self.Character`) _returnvalue_2 false))
  (for _array_element _returnvalue_4
    (bind _output_get (set `local.MapCell` _array_element))
    (bind _returnvalue_5 (message `AreaModifierInterface.GetStatusForTile` (`self.Character`) (`.Character` (break `MapCell` _output_get))))
    (`KKTile.SetTileStatus` _mapcell_tile _returnvalue_5)
    (`/Engine/EditorBlueprintResources/StandardMacros.IsValid` (`.Character` (break `MapCell` _output_get))
      (:`Is Valid`
        (`KismetArrayLibrary.Array_Add` (`self.AffectedCharacters`) (`.Character` (break `MapCell` _output_get))))))
  (`self.SetAffectedCharacters` (`self.AffectedCharacters`)))

(fn `UserConstructionScript`
  (`parent.UserConstructionScript`))