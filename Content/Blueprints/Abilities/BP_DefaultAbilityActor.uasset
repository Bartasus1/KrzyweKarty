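; Default ability actor that handles confirm and abort input for a character ability.
; Confirm calls ConfirmAbility when CanFinishAbility passes, otherwise OnAbilityFailedToFinish, while abort calls AbortAbility.
; After a successful confirm or an abort, BP_KKPlayerController turns off character ability input and restores the character selection input tag.
; CanFinishAbility returns true and the failure hook is empty, serving as default implementations.
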(event `EnhancedInput|/Game/Player/Input/Actions/IA_Confirm`
  (params (ActionValue :type Boolean) (ElapsedSeconds :type "Float (double-precision)") (TriggeredSeconds :type "Float (double-precision)") (InputAction :type "InputAction Object Reference" :default "/Game/Player/Input/Actions/IA_Confirm.IA_Confirm"))
  (bind _asbp_kkplayer_controller (cast `/Game/Player/BP_KKPlayerController` (`GameplayStatics.GetPlayerController` 0) :!pure true))
  (:`Completed`
    (if (`self.CanFinishAbility?`)
      (`self.ConfirmAbility`)
      (`/Game/Player/BP_KKPlayerController.Manage Character Ability Input` _asbp_kkplayer_controller false :!label _label)
      (set `/Game/Player/BP_KKPlayerController.SelectionInputTag` (struct :`TagName` "Selection.CharacterSelection") _asbp_kkplayer_controller)
      (else
        (`self.OnAbilityFailedToFinish`)))))

(event `EnhancedInput|/Game/Player/Input/Actions/IA_Abort`
  (params (ActionValue :type Boolean) (ElapsedSeconds :type "Float (double-precision)") (TriggeredSeconds :type "Float (double-precision)") (InputAction :type "InputAction Object Reference" :default "/Game/Player/Input/Actions/IA_Abort.IA_Abort"))
  (:`Completed`
    (`self.AbortAbility`)
    (goto _label)))

(fn `CanFinishAbility?`
  (returns (`Can Finish` :type Boolean))
  (return true))

(fn `OnAbilityFailedToFinish`)

(fn `UserConstructionScript`)